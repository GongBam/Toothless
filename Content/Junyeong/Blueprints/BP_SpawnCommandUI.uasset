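; BP_SpawnCommandUI is a VR command menu actor that animates a 3D CommandUI widget open and closed.
; BeginPlay adds the IMC_Menu input context, caches the active hand's aim controller and plays a timeline that scales up the widget.
; CommandClose removes the context and reverses the timeline, then attempts to snap the widget interaction component to that controller.
; Its interaction-component lookup is incomplete: the right reference is assigned None and the left is unset.
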(event `self.ReceiveBeginPlay`
  (bind _relativescale3d_x (`KismetMathLibrary.BreakVector` (`SceneComponent.RelativeScale3D` (`self.CommandUI`))))
  (`self.EnableInput` (`GameplayStatics.GetPlayerController` 0))
  (message `EnhancedInputSubsystemInterface.AddMappingContext` (pcsubsystem `EnhancedInputLocalPlayerSubsystem` (`GameplayStatics.GetPlayerController` 0)) "/Game/VRTemplate/Input/IMC_Menu.IMC_Menu" 0 (struct))
  (`self.SetWidgetInteractionReferences`)
  (`self.SetMotionControllerReference`)
  (set `self.WidgetRelativeScaleOriginal` _relativescale3d_x)
  (bind (_direction _alpha) (`Timeline|OpenMenuAnmiationTimeline` :!label _label)
    (:`Update`
      (`SceneComponent.SetRelativeScale3D` (`self.CommandUI`) (`KismetMathLibrary.Conv_DoubleToVector` (* _alpha (`self.WidgetRelativeScaleOriginal`)))))
    (:`Finished`
      (if (`|EnumEquality` _direction "Backward")
        (`SceneComponent.K2_AttachToComponent` (`self.GetWidgetInteractionComponent` (`self.bActiveMenuHandRight`)) (`self.MotionControllerAimRef`) "None" "SnapToTarget" "SnapToTarget" "KeepWorld" true)))))

(event `Command Close`
  (`EnhancedInputSubsystemInterface.RemoveMappingContext` (pcsubsystem `EnhancedInputLocalPlayerSubsystem` (`GameplayStatics.GetPlayerController` 0)) "/Game/VRTemplate/Input/IMC_Menu.IMC_Menu" (struct))
  (goto _label :!via `Reverse`))

(fn `GetWidgetInteractionComponent`
  (params (bRightWIC :type Boolean))
  (returns (ReturnValue :type "WidgetInteractionComponent Object Reference"))
  (return (select `bool` bRightWIC :`true` (`self.WidgetInteractionRefRight`))))

(fn `SetMotionControllerReference`
  (locals (LocalMotionControllers :type "Array of MotionControllerComponent Object Reference"))
  (bind _returnvalue (`self.K2_GetComponentsByClass` (`GameplayStatics.GetPlayerPawn` 0) "/Script/HeadMountedDisplay.MotionControllerComponent"))
  (if (> (`KismetArrayLibrary.Array_Length` _returnvalue) 0)
    (bind _output_get (set `local.LocalMotionControllers` _returnvalue))
    (for _array_element _output_get
      (if (== (`MotionControllerComponent.MotionSource` _array_element) (select `bool` (`self.bActiveMenuHandRight`) :`false` "LeftAim" :`true` "RightAim" :!type "Name"))
        (set `self.MotionControllerAimRef` _array_element)))))

(fn `SetWidgetInteractionReferences`
  (locals (LocalWidgetInteractionComponents :type "Array of WidgetInteractionComponent Object Reference"))
  (bind _returnvalue (`self.K2_GetComponentsByClass` (`GameplayStatics.GetPlayerPawn` 0) "/Script/UMG.WidgetInteractionComponent"))
  (if (> (`KismetArrayLibrary.Array_Length` _returnvalue) 0)
    (bind _output_get (set `local.LocalWidgetInteractionComponents` _returnvalue))
    (for _array_element _output_get
      (if (== (`WidgetInteractionComponent.PointerIndex` _array_element) 0)
        (set `self.WidgetInteractionRefRight` null)))))

(fn `UserConstructionScript`)
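; Rideable flying character for the happy-ending sequence, which carries the player through the sky and then loads DemoMap.
; Sphere overlap with a VRPawn calls that pawn's Dartride.
; Ride possesses this character, loops a flying animation, teleports it high up, drives it along Y with a timeline and opens the level after a delay.
; A dartmoveto event sets walk speed and issues a simple move through the player controller.
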(event `/Game/Happyendingrid/bp_ride.Ride`
  (bind (_returnvalue_x _returnvalue_y _returnvalue_z) (`KismetMathLibrary.BreakVector` (`self.K2_GetActorLocation`)))
  (set `self.isride` true)
  (`Controller.Possess` (`GameplayStatics.GetPlayerController` 0) self)
  (`self.PlayAnimMontage` null)
  (`SkeletalMeshComponent.PlayAnimation` (`self.Mesh`) "/Game/dartanimation/animbasicfly.animbasicfly" true)
  (`KismetSystemLibrary.Delay` 0.5)
  (`self.K2_SetActorLocationAndRotation` (-9740.0 -4880.0 20000.0) (`self.K2_GetActorRotation`))
  (bind (_direction _newtrack_0) (`Timeline|Timeline` :!via `PlayFromStart`)
    (:`Update`
      (`self.K2_SetActorLocation` (`KismetMathLibrary.MakeVector` _returnvalue_x (+ _newtrack_0 _returnvalue_y) _returnvalue_z))
      (`KismetSystemLibrary.Delay` 14.0)
      (`GameplayStatics.OpenLevel` "DemoMap"))))

(event `dart move to`
  (params (Location :type "Vector Structure") (speed :type "Float (double-precision)") (normalspeed :type "Float (double-precision)"))
  (set `CharacterMovementComponent.MaxWalkSpeed` speed (`self.CharacterMovement`))
  (`AIBlueprintHelperLibrary.SimpleMoveToLocation` (`GameplayStatics.GetPlayerController` 0) Location))

(event `self.Sphere.OnComponentBeginOverlap`
  (params (OverlappedComponent :type "PrimitiveComponent Object Reference") (OtherActor :type "Actor Object Reference") (OtherComp :type "PrimitiveComponent Object Reference") (OtherBodyIndex :type Integer) (bFromSweep :type Boolean) (SweepResult :type "HitResult Structure (by ref)"))
  (bind _asvrpawn (cast `/Game/VRTemplate/Blueprints/VRPawn` OtherActor))
  (`/Game/VRTemplate/Blueprints/VRPawn.dartride` _asvrpawn))

(fn `UserConstructionScript`)